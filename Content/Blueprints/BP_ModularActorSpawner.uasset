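; Modular spawner that creates actors of a configurable class at target points, starting on BeginPlay or on a one-shot player box overlap.
; Each spawn picks a random point, or in shuffle mode walks the array and reshuffles once exhausted.
; An invalid point in shuffle mode refills the array with every TargetPoint in the level.
; Optional looping repeats spawns after a delay, up to a limit.
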(event OnComponentBeginOverlap(Box)
  (params (OverlappedComponent :type Primitive%20Component%20Object%20Reference) (OtherActor :type Actor%20Object%20Reference) (OtherComp :type Primitive%20Component%20Object%20Reference) (OtherBodyIndex :type Integer) (bFromSweep :type Boolean) (SweepResult :type Hit%20Result%20Structure%20%28by%20ref%29))
  ;[0.15 0.15 0.15 0.5] Start spawning on begin play or on box collision?
  (Utilities|Casting|CastToBPC_PlayerCharacter OtherActor)
  (if (Variables|Default|GetbUseOverlapTrigger)
    (CallFunction|StartSpawn)
    (Components|DestroyComponent (Variables|Default|GetBox))))

(event Custom|StartLoopingSpawn
  ;[0.15 0.15 0.15 0.5] Loop Spawn
  (if (< (Variables|Default|GetLoopSpawnCounter) (Variables|Default|GetLoopSpawnLimit))
    (Math|Integer|IncrementInt (Variables|Default|GetLoopSpawnCounter)
      (:%20%20
        (Utilities|FlowControl|Delay (Variables|Default|GetLoopSpawnInterval))
        ;[0.15 0.15 0.15 0.5] Validation
        (if (and (Utilities|IsValidClass (Variables|Default|GetSpawnClass)) (Utilities|Array|IsNotEmpty (Variables|Default|GetTargetPoints)))
          (if (Variables|Default|GetbUseShuffledSpawn)
            (if (>= (Variables|Default|GetShuffleIndex) (Utilities|Array|Length (Variables|Default|GetTargetPoints)))
              ;[0.15 0.15 0.15 0.5] Shuffle and Reset
              (Utilities|Array|Shuffle (Variables|Default|GetTargetPoints))
              (Variables|Default|SetShuffleIndex 0))
            (Utilities|IsValid (Utilities|Array|Get(acopy) (Variables|Default|GetTargetPoints) (Variables|Default|GetShuffleIndex))
              (:Is%20Valid
                ;[0.15 0.15 0.15 0.5] Spawn Shuffled Actor
                (Game|SpawnActorfromClass (Variables|Default|GetSpawnClass) (Transformation|GetActorTransform (Utilities|Array|Get(acopy) (Variables|Default|GetTargetPoints) (Variables|Default|GetShuffleIndex))) "Undefined" "MultiplyWithRoot" 0 0))
              (:Is%20Not%20Valid
                ;[0.15 0.15 0.15 0.5] Reset the array if a target point is missing.
                (bind _outactors (Actor|GetAllActorsOfClass "/Script/Engine.TargetPoint"))
                (Variables|Default|SetTargetPoints _outactors)))
            (else
              ;[0.15 0.15 0.15 0.5] Spawn Random Actor
              (Game|SpawnActorfromClass (Variables|Default|GetSpawnClass) (Transformation|GetActorTransform (.OutItem (Utilities|Array|Random (Variables|Default|GetTargetPoints)))) "Undefined" "MultiplyWithRoot" 0 0)))
          (Math|Integer|IncrementInt (Variables|Default|GetShuffleIndex)
            (:%20%20
              (if (Variables|Default|GetbLoopSpawn)
                (CallFunction|StartLoopingSpawn))))
          (else
            (Development|PrintString "BP_ModularRandomSpawner failed to validate the variables." true true "(R=1.000000,G=0.000000,B=0.000000,A=1.000000)" 5.0)))))))

(event Custom|StartSpawn
  ;[0.15 0.15 0.15 0.5] Validation
  (if (and (Utilities|IsValidClass (Variables|Default|GetSpawnClass)) (Utilities|Array|IsNotEmpty (Variables|Default|GetTargetPoints)))
    (if (Variables|Default|GetbUseShuffledSpawn)
      (if (>= (Variables|Default|GetShuffleIndex) (Utilities|Array|Length (Variables|Default|GetTargetPoints)))
        ;[0.15 0.15 0.15 0.5] Shuffle and Reset
        (Utilities|Array|Shuffle (Variables|Default|GetTargetPoints))
        (Variables|Default|SetShuffleIndex 0))
      (Utilities|IsValid (Utilities|Array|Get(acopy) (Variables|Default|GetTargetPoints) (Variables|Default|GetShuffleIndex))
        (:Is%20Valid
          ;[0.15 0.15 0.15 0.5] Spawn Shuffled Actor
          (Game|SpawnActorfromClass (Variables|Default|GetSpawnClass) (Transformation|GetActorTransform (Utilities|Array|Get(acopy) (Variables|Default|GetTargetPoints) (Variables|Default|GetShuffleIndex))) "Undefined" "MultiplyWithRoot" 0 0))
        (:Is%20Not%20Valid
          ;[0.15 0.15 0.15 0.5] Reset the array if a target point is missing.
          (bind _outactors (Actor|GetAllActorsOfClass "/Script/Engine.TargetPoint"))
          (Variables|Default|SetTargetPoints _outactors)))
      (else
        ;[0.15 0.15 0.15 0.5] Spawn Random Actor
        (Game|SpawnActorfromClass (Variables|Default|GetSpawnClass) (Transformation|GetActorTransform (.OutItem (Utilities|Array|Random (Variables|Default|GetTargetPoints)))) "Undefined" "MultiplyWithRoot" 0 0)))
    (Math|Integer|IncrementInt (Variables|Default|GetShuffleIndex)
      (:%20%20
        ;[0.15 0.15 0.15 0.5] Loop Spawn
        (if (Variables|Default|GetbLoopSpawn)
          (CallFunction|StartLoopingSpawn))))
    (else
      (Development|PrintString "BP_ModularRandomSpawner failed to validate the variables." true true "(R=1.000000,G=0.000000,B=0.000000,A=1.000000)" 5.0))))

(event EventBeginPlay
  ;[0.15 0.15 0.15 0.5] Start spawning on begin play or on box collision?
  (if (not (Variables|Default|GetbUseOverlapTrigger))
    (CallFunction|StartSpawn)))

(event EventTick
  (params (DeltaSeconds :type Float%20%28single-precision%29)))

(fn ConstructionScript)