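; Player character Blueprint that handles basic movement through Enhanced Input.
; BeginPlay adds the movement mapping context to the local player subsystem of player controller 0.
; IA_Movement feeds its X and Y values into movement along fixed world X and Y axes, independent of camera or control rotation.
; That input is applied only when the health component's Alive flag is false.
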(event Input|EnhancedActionEvents|EnhancedInputActionIA_Movement
  (params (ActionValue :type Vector%202D%20Structure) (ElapsedSeconds :type Float%20%28double-precision%29) (TriggeredSeconds :type Float%20%28double-precision%29) (InputAction :type Input%20Action%20Object%20Reference :default "/Game/Blueprints/Gameplay/Inputs/IA_Movement.IA_Movement"))
  (bind (_x _y) (Math|Vector2D|BreakVector2D ActionValue))
  (if (not (Variables|/Game/Blueprints/Components/AC_Health.AC_Health_C|GetbAlive (Variables|Default|GetAC_Health)))
    (Pawn|Input|AddMovementInput "1.000000,0.000000,0.000000" _x false)
    (Pawn|Input|AddMovementInput "0.000000,1.000000,0.000000" _y false)))

(event EventBeginPlay
  (Input|AddMappingContext (PlayerController|LocalPlayerSubsystems|GetEnhancedInputLocalPlayerSubsystem (Game|GetPlayerController 0)) "/Game/Blueprints/Gameplay/Inputs/IMC_MovementMapping.IMC_MovementMapping" 0 "(bIgnoreAllPressedKeysUntilRelease=True,bForceImmediately=False,bNotifyUserSettings=False)"))

(event Collision|EventActorBeginOverlap
  (params (OtherActor :type Actor%20Object%20Reference)))

(event EventTick
  (params (DeltaSeconds :type Float%20%28single-precision%29)))

(fn ConstructionScript
  (|CallParentFunction))